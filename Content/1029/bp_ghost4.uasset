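; Afterimage actor that leaves a frozen ghost of the player character's pose as a trail effect.
; On BeginPlay, GhostTrailS2 gives the poseable mesh dynamic GhostMat8 materials, copies the player's current pose and starts an opacity timeline.
; The timeline is set up to drive the materials' opacity parameters and destroy the actor when finished.
; GhostTarils is a GhostMat7 variant that nothing in this graph calls.
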(event `self.ReceiveBeginPlay`
  (`self.GhostTrailS2`))

(event `GhostTarils`
  (for _ (`MeshComponent.GetMaterials` (`self.PoseableMesh`))
    (bind _returnvalue (`KismetMaterialLibrary.CreateDynamicMaterialInstance` "/Game/1029/GhostMat7.GhostMat7" "None" "Transient"))
    (bind _returnvalue_2 (`KismetArrayLibrary.Array_Add` (`self.DynamicMat`) _returnvalue))
    (`PrimitiveComponent.SetMaterial` (`self.PoseableMesh`) _returnvalue_2 _returnvalue)
    (`PoseableMeshComponent.CopyPoseFromSkeletalComponent` (`self.PoseableMesh`) (`Character.Mesh` (`self.Playerchar`)))
    (`TimelineComponent.PlayFromStart` (`self.OParCity_Template`))))

(event `GhostTrailS2`
  (for _ (`MeshComponent.GetMaterials` (`self.PoseableMesh`))
    (bind _returnvalue (`KismetMaterialLibrary.CreateDynamicMaterialInstance` "/Game/1029/GhostMat8.GhostMat8" "None" "Transient"))
    (bind _returnvalue_2 (`KismetArrayLibrary.Array_Add` (`self.DynamicMat`) _returnvalue))
    (`PrimitiveComponent.SetMaterial` (`self.PoseableMesh`) _returnvalue_2 _returnvalue)
    (`PoseableMeshComponent.CopyPoseFromSkeletalComponent` (`self.PoseableMesh`) (`Character.Mesh` (`self.Playerchar`)))
    (`TimelineComponent.PlayFromStart` (`self.OParCity_Template`))))

(fn `UserConstructionScript`)